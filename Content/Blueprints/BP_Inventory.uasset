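; BP_Inventory is an inventory Blueprint with functions to add, remove and find items in a Content collection.
; Add copies the requested quantity into a remaining counter and loops while it is positive, but the loop body is empty.
; Remove deletes the Content entry at the given Id.
; FindItem iterates Content with an empty body, leaving the element Name unused, so no search result is produced.
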(fn Add
  (params (item :type Name) (Quantity :type Integer))
  (LocalVariables|SetLocal_QuantityRemaining Quantity)
  (while (> (LocalVariables|GetLocal_QuantityRemaining) 0)
    _))

(fn Remove
  (params (id :type Integer))
  (Utilities|Array|RemoveItem (Variables|Default|GetContent) (Utilities|Array|Get(acopy) (Variables|Default|GetContent) id)))

(fn FindItem
  (params (ItemName :type Name))
  (for _array_element (Variables|Default|GetContent)
    _))