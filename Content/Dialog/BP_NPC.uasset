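; BP_NPC is an NPC Blueprint that shows its dialogue lines one at a time on screen.
; Each Talk event increments TalkIndex, creates and caches a WB_Dialog widget if needed, sets its text from the Dialog array and plays a 2D sound.
; When the index passes the last line, it resets and loops back to show the first line again.
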(event EventTalk
  (Math|Integer|IncrementInt (Variables|Default|GetTalk%20Index) :!label _label
    (:%20%20
      (if (< (Variables|Default|GetTalk%20Index) (Utilities|Array|Length (Variables|Default|GetDialog)))
        (Variables|Default|GetUI
          (:then
            _)
          (:else
            (bind _returnvalue (Game|ConstructObjectfromClass (Game|GetPlayerController 0) "/Game/Dialog/WB_Dialog.WB_Dialog_C"))
            (bind _output_get (Variables|Default|SetUI _returnvalue))
            (UserInterface|Viewport|AddtoViewport _output_get 0)))
        (Rendering|Components|TextRender|SetText (Variables|/Game/Dialog/WB_Dialog.WB_Dialog_C|GetTextTalk (Variables|Default|GetUI)) (Utilities|Text|ToText(String) (Utilities|Array|Get(acopy) (Variables|Default|GetDialog) (Variables|Default|GetTalk%20Index))))
        (Audio|PlaySound2D 0 1.0 1.0 0.0 0 0)
        (elif (== (Variables|Default|GetTalk%20Index) (Utilities|Array|Length (Variables|Default|GetDialog)))
          (Variables|Default|SetTalk%20Index -1)
          (goto _label))))))

(fn ConstructionScript)